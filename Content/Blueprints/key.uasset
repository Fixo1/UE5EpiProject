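; Key item actor that the player can interact with when standing inside its sphere trigger.
; On overlap by the player character it shows an InteractMsg widget with the item's name and text, then sets BP_MyCharacter's near-item flag, interact type and item reference to itself.
; When an overlap ends while the widget is valid, it removes the prompt and clears only the character's near-item flag.
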(event OnComponentBeginOverlap(Sphere)
  (params (OverlappedComponent :type Primitive%20Component%20Object%20Reference) (OtherActor :type Actor%20Object%20Reference) (OtherComp :type Primitive%20Component%20Object%20Reference) (OtherBodyIndex :type Integer) (bFromSweep :type Boolean) (SweepResult :type Hit%20Result%20Structure%20%28by%20ref%29))
  (if (== OtherActor (Game|GetPlayerCharacter 0))
    (bind _returnvalue (UserInterface|CreateWidget "/Game/Blueprints/interactMsg.interactMsg_C" 0 (Variables|Default|GetName%20Of%20Item) (Variables|Default|GetText%20to%20Display)))
    (bind _output_get (Variables|Default|SetinteractUI _returnvalue))
    (UserInterface|Viewport|AddtoViewport _output_get 0)
    (bind _asbp_my_character (Utilities|Casting|CastToBP_MyCharacter OtherActor))
    (Variables|/Game/Blueprints/BP_MyCharacter.BP_MyCharacter_C|SetnearAnItem _asbp_my_character true)
    (Variables|/Game/Blueprints/BP_MyCharacter.BP_MyCharacter_C|SetenumInteractItem _asbp_my_character "NewEnumerator1")
    (Variables|/Game/Blueprints/BP_MyCharacter.BP_MyCharacter_C|SetinteractItem _asbp_my_character self)))

(event OnComponentEndOverlap(Sphere)
  (params (OverlappedComponent :type Primitive%20Component%20Object%20Reference) (OtherActor :type Actor%20Object%20Reference) (OtherComp :type Primitive%20Component%20Object%20Reference) (OtherBodyIndex :type Integer))
  (bind _interactui (Variables|Default|GetinteractUI))
  (Utilities|IsValid _interactui
    (:Is%20Valid
      (Widget|RemovefromParent _interactui)
      (bind _asbp_my_character (Utilities|Casting|CastToBP_MyCharacter OtherActor))
      (Variables|/Game/Blueprints/BP_MyCharacter.BP_MyCharacter_C|SetnearAnItem _asbp_my_character false))))

(fn ConstructionScript)