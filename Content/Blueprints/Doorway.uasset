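; Doorway Blueprint that swings a large two-leaf door open when the openDoor event is called.
; openDoor starts a fast looping timer on rotateDoor, which eases each leaf's yaw toward its target with FInterpTo.
; Targets are fixed world-space yaws set slightly past the stop thresholds, and the timer clears once both interpolated values reach those thresholds.
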(event Custom|openDoor
  (Utilities|Time|SetTimerbyFunctionName 0 "rotateDoor" 0.01 true))

(fn ConstructionScript)

(fn RotateDoor
  (bind _returnvalue (Utilities|Time|GetWorldDeltaSeconds))
  (bind _sm_doorway_large_door_left (Variables|Default|GetSM_DoorWay_Large_Door_Left))
  (bind _sm_doorway_large_door_right (Variables|Default|GetSM_DoorWay_Large_Door_Right))
  (bind _returnvalue_2 (Transformation|GetWorldRotation _sm_doorway_large_door_right))
  (bind _returnvalue_3 (Transformation|GetWorldRotation _sm_doorway_large_door_left))
  (bind _returnvalue_4 (Math|Interpolation|FInterpTo (.yaw _returnvalue_3) 185.0 _returnvalue 0.3))
  (bind _returnvalue_5 (Math|Interpolation|FInterpTo (.yaw _returnvalue_2) -5.0 _returnvalue 0.3))
  (Transformation|SetWorldRotation (Variables|Default|GetSM_DoorWay_Large_Door_Left) (Math|Rotator|MakeRotator 0.0 0.0 _returnvalue_4) false false)
  (Transformation|SetWorldRotation (Variables|Default|GetSM_DoorWay_Large_Door_Right) (Math|Rotator|MakeRotator 0.0 0.0 _returnvalue_5) false false)
  (if (and (>= _returnvalue_4 1.8e+02) (<= _returnvalue_5 0.0))
    (Utilities|Time|ClearTimerbyFunctionName 0 "rotateDoor")))