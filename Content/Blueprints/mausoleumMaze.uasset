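; Mausoleum maze puzzle actor where a stone lid is shifted between positions on a grid, four across and three high.
; Four shift events step clamped X and Y indices, then teleport the lid and play a stone slide sound.
; Height is offset from the first origin marker, while each column snaps to its own marker with an added yaw step, forming an arc.
; The isWin event opens the Door when the lid sits at the winning cell.
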(event Custom|shiftRight
  (bind _lid (Variables|Default|Getlid))
  (bind _lid_origin0 (Variables|Default|Getlid_origin0))
  (bind _lid_origin1 (Variables|Default|Getlid_origin1))
  (bind _lid_origin2 (Variables|Default|Getlid_origin2))
  (bind _lid_origin3 (Variables|Default|Getlid_origin3))
  (bind _returnvalue (Transformation|GetWorldLocation _lid_origin0))
  (bind _returnvalue_2 (Transformation|GetWorldLocation _lid_origin3))
  (bind _returnvalue_3 (Transformation|GetWorldLocation _lid_origin2))
  (bind _returnvalue_4 (Transformation|GetWorldLocation _lid_origin1))
  (bind _returnvalue_5 (Transformation|GetWorldRotation _lid))
  (if (< (Variables|Default|Getx) 3)
    (Variables|Default|Setx (+ 1 (Variables|Default|Getx)))
    (Transformation|SetWorldRotation (Variables|Default|Getlid) (Math|Rotator|MakeRotator (.roll _returnvalue_5) (.pitch _returnvalue_5) (+ (.yaw (Transformation|GetWorldRotation (Variables|Default|Getlid_origin0))) (* (Variables|Default|Getx) 20))) false true)
    (if (== 0 (Variables|Default|Getx))
      (Transformation|SetWorldLocation (Variables|Default|Getlid) (Math|Vector|MakeVector (.x _returnvalue) (.y _returnvalue) (.z (Transformation|GetWorldLocation (Variables|Default|Getlid)))) false true)
      (Audio|PlaySoundatLocation "/Game/sounds/stoneSlide.stoneSlide" (Transformation|GetWorldLocation (Variables|Default|Getlid)) "0, 0, 0" 1.0 1.0 0.0 0 0 0 0 :!label _label)
      (elif (== 1 (Variables|Default|Getx))
        (Transformation|SetWorldLocation (Variables|Default|Getlid) (Math|Vector|MakeVector (.x _returnvalue_4) (.y _returnvalue_4) (.z (Transformation|GetWorldLocation (Variables|Default|Getlid)))) false true)
        (goto _label)
        (elif (== 2 (Variables|Default|Getx))
          (Transformation|SetWorldLocation (Variables|Default|Getlid) (Math|Vector|MakeVector (.x _returnvalue_3) (.y _returnvalue_3) (.z (Transformation|GetWorldLocation (Variables|Default|Getlid)))) false true)
          (goto _label)
          (elif (== 3 (Variables|Default|Getx))
            (Transformation|SetWorldLocation (Variables|Default|Getlid) (Math|Vector|MakeVector (.x _returnvalue_2) (.y _returnvalue_2) (.z (Transformation|GetWorldLocation (Variables|Default|Getlid)))) false true)
            (goto _label)))))))

(event Custom|shiftLeft
  (bind _lid (Variables|Default|Getlid))
  (bind _lid_origin0 (Variables|Default|Getlid_origin0))
  (bind _lid_origin1 (Variables|Default|Getlid_origin1))
  (bind _lid_origin2 (Variables|Default|Getlid_origin2))
  (bind _lid_origin3 (Variables|Default|Getlid_origin3))
  (bind _returnvalue (Transformation|GetWorldLocation _lid_origin0))
  (bind _returnvalue_2 (Transformation|GetWorldLocation _lid_origin3))
  (bind _returnvalue_3 (Transformation|GetWorldLocation _lid_origin2))
  (bind _returnvalue_4 (Transformation|GetWorldLocation _lid_origin1))
  (bind _returnvalue_5 (Transformation|GetWorldRotation _lid))
  (if (> (Variables|Default|Getx) 0)
    (Variables|Default|Setx (+ -1 (Variables|Default|Getx)))
    (Transformation|SetWorldRotation (Variables|Default|Getlid) (Math|Rotator|MakeRotator (.roll _returnvalue_5) (.pitch _returnvalue_5) (+ (.yaw (Transformation|GetWorldRotation (Variables|Default|Getlid_origin0))) (* (Variables|Default|Getx) 20))) false true)
    (if (== 0 (Variables|Default|Getx))
      (Transformation|SetWorldLocation (Variables|Default|Getlid) (Math|Vector|MakeVector (.x _returnvalue) (.y _returnvalue) (.z (Transformation|GetWorldLocation (Variables|Default|Getlid)))) false true)
      (Audio|PlaySoundatLocation "/Game/sounds/stoneSlide.stoneSlide" (Transformation|GetWorldLocation (Variables|Default|Getlid)) "0, 0, 0" 1.0 1.0 0.0 0 0 0 0 :!label _label)
      (elif (== 1 (Variables|Default|Getx))
        (Transformation|SetWorldLocation (Variables|Default|Getlid) (Math|Vector|MakeVector (.x _returnvalue_4) (.y _returnvalue_4) (.z (Transformation|GetWorldLocation (Variables|Default|Getlid)))) false true)
        (goto _label)
        (elif (== 2 (Variables|Default|Getx))
          (Transformation|SetWorldLocation (Variables|Default|Getlid) (Math|Vector|MakeVector (.x _returnvalue_3) (.y _returnvalue_3) (.z (Transformation|GetWorldLocation (Variables|Default|Getlid)))) false true)
          (goto _label)
          (elif (== 3 (Variables|Default|Getx))
            (Transformation|SetWorldLocation (Variables|Default|Getlid) (Math|Vector|MakeVector (.x _returnvalue_2) (.y _returnvalue_2) (.z (Transformation|GetWorldLocation (Variables|Default|Getlid)))) false true)
            (goto _label)))))))

(event Custom|shiftUp
  (bind _lid (Variables|Default|Getlid))
  (bind _returnvalue (Transformation|GetWorldLocation _lid))
  (if (< (Variables|Default|Gety) 2)
    (Variables|Default|Sety (+ 1 (Variables|Default|Gety)))
    (Transformation|SetWorldLocation (Variables|Default|Getlid) (Math|Vector|MakeVector (.x _returnvalue) (.y _returnvalue) (+ (.z (Transformation|GetWorldLocation (Variables|Default|Getlid_origin0))) (* (Variables|Default|Gety) 120))) false true)
    (Audio|PlaySoundatLocation "/Game/sounds/stoneSlide.stoneSlide" (Transformation|GetWorldLocation (Variables|Default|Getlid)) "0, 0, 0" 1.0 1.0 0.0 0 0 0 0)))

(event Custom|shiftDown
  (bind _lid (Variables|Default|Getlid))
  (bind _returnvalue (Transformation|GetWorldLocation _lid))
  (if (> (Variables|Default|Gety) 0)
    (Variables|Default|Sety (+ -1 (Variables|Default|Gety)))
    (Transformation|SetWorldLocation (Variables|Default|Getlid) (Math|Vector|MakeVector (.x _returnvalue) (.y _returnvalue) (+ (.z (Transformation|GetWorldLocation (Variables|Default|Getlid_origin0))) (* (Variables|Default|Gety) 120))) false true)
    (Audio|PlaySoundatLocation "/Game/sounds/stoneSlide.stoneSlide" (Transformation|GetWorldLocation (Variables|Default|Getlid)) "0, 0, 0" 1.0 1.0 0.0 0 0 0 0)))

(event Custom|isWin
  (if (== (Variables|Default|Getx) 3)
    (if (== (Variables|Default|Gety) 1)
      (Default|OpenDoor (Variables|Default|Getdoor)))))

(fn ConstructionScript)