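; Cell door actor that the player can open when it is not locked and the player holds a key.
; Its box overlap shows an interaction message widget and registers the door as the nearby interact item on BP_MyCharacter; leaving removes the prompt.
; The openDoor event starts a looping timer on rotateDoor, which interpolates the mesh's world yaw toward 90 degrees and clears itself near the end.
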(event OnComponentBeginOverlap(Box)
  (params (OverlappedComponent :type Primitive%20Component%20Object%20Reference) (OtherActor :type Actor%20Object%20Reference) (OtherComp :type Primitive%20Component%20Object%20Reference) (OtherBodyIndex :type Integer) (bFromSweep :type Boolean) (SweepResult :type Hit%20Result%20Structure%20%28by%20ref%29))
  (if (== OtherActor (Game|GetPlayerCharacter 0))
    (bind _returnvalue (UserInterface|CreateWidget "/Game/Blueprints/interactMsg.interactMsg_C" 0 (Variables|Default|GetName%20Of%20Item) (Variables|Default|GetText%20to%20Display)))
    (bind _output_get (Variables|Default|SetinteractUI _returnvalue))
    (UserInterface|Viewport|AddtoViewport _output_get 0)
    (bind _asbp_my_character (Utilities|Casting|CastToBP_MyCharacter OtherActor))
    (Variables|/Game/Blueprints/BP_MyCharacter.BP_MyCharacter_C|SetnearAnItem _asbp_my_character true)
    (Variables|/Game/Blueprints/BP_MyCharacter.BP_MyCharacter_C|SetenumInteractItem _asbp_my_character "NewEnumerator0")
    (Variables|/Game/Blueprints/BP_MyCharacter.BP_MyCharacter_C|SetinteractItem _asbp_my_character self)))

(event OnComponentEndOverlap(Box)
  (params (OverlappedComponent :type Primitive%20Component%20Object%20Reference) (OtherActor :type Actor%20Object%20Reference) (OtherComp :type Primitive%20Component%20Object%20Reference) (OtherBodyIndex :type Integer))
  (bind _interactui (Variables|Default|GetinteractUI))
  (Utilities|IsValid _interactui
    (:Is%20Valid
      (Widget|RemovefromParent _interactui)
      (bind _asbp_my_character (Utilities|Casting|CastToBP_MyCharacter OtherActor))
      (Variables|/Game/Blueprints/BP_MyCharacter.BP_MyCharacter_C|SetnearAnItem _asbp_my_character false))))

(event Custom|openDoor
  (if (not (Variables|Default|GetisLocked))
    (bind _asbp_my_character (Utilities|Casting|CastToBP_MyCharacter (Game|GetPlayerCharacter 0)))
    (if (Variables|/Game/Blueprints/BP_MyCharacter.BP_MyCharacter_C|GethasKey _asbp_my_character)
      (Utilities|Time|SetTimerbyFunctionName 0 "rotateDoor" 0.01 true))))

(fn ConstructionScript)

(fn RotateDoor
  (bind _returnvalue (Utilities|Time|GetWorldDeltaSeconds))
  (bind _sm_cell_door (Variables|Default|GetSM_Cell_Door))
  (bind _returnvalue_2 (Transformation|GetWorldRotation _sm_cell_door))
  (bind _returnvalue_3 (Math|Interpolation|FInterpTo (.yaw _returnvalue_2) 9e+01 _returnvalue 0.3))
  (Transformation|SetWorldRotation (Variables|Default|GetSM_Cell_Door) (Math|Rotator|MakeRotator 0.0 0.0 _returnvalue_3) false false)
  (if (>= _returnvalue_3 88.0)
    (Utilities|Time|ClearTimerbyFunctionName 0 "rotateDoor")))