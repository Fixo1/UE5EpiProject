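; BP_Target is a moving target that awards points and plays an explosion sound when a BP_Arrow overlaps its TargetBox.
; On BeginPlay, two chained timelines lerp it back and forth along Y from its starting location in an endless loop.
; Points go to CharacterRef only when it is valid, and BeginPlay assigns the player character to it only if it is already valid.
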(event OnComponentBeginOverlap(TargetBox)
  (params (OverlappedComponent :type Primitive%20Component%20Object%20Reference) (OtherActor :type Actor%20Object%20Reference) (OtherComp :type Primitive%20Component%20Object%20Reference) (OtherBodyIndex :type Integer) (bFromSweep :type Boolean) (SweepResult :type Hit%20Result%20Structure%20%28by%20ref%29))
  (bind _characterref (Variables|Default|GetCharacterRef))
  (Utilities|Casting|CastToBP_Arrow OtherActor)
  (Utilities|IsValid _characterref
    (:Is%20Valid
      (Variables|/Game/Blueprints/BP_MyCharacter.BP_MyCharacter_C|SetPoints _characterref (+ (Variables|/Game/Blueprints/BP_MyCharacter.BP_MyCharacter_C|GetPoints _characterref) 10))
      (Audio|PlaySoundatLocation "/Game/StarterContent/Audio/Explosion01.Explosion01" (Transformation|GetActorLocation) "0, 0, 0" 1.0 1.0 0.0 0 0 0 0))
    (:Is%20Not%20Valid
      (Audio|PlaySoundatLocation "/Game/StarterContent/Audio/Explosion01.Explosion01" (Transformation|GetActorLocation) "0, 0, 0" 1.0 1.0 0.0 0 0 0 0))))

(event EventBeginPlay
  (bind _returnvalue (Transformation|GetActorLocation))
  (Variables|Default|SetStart (Math|Vector|MakeVector (.x _returnvalue) (.y _returnvalue) (.z _returnvalue)))
  (Variables|Default|SetEnd (Math|Vector|MakeVector (.x _returnvalue) (- (.y _returnvalue) 3e+02) (.z _returnvalue)))
  (Utilities|IsValid (stale _output_get)
    (:Is%20Valid
      (bind _asbp_my_character (Utilities|Casting|CastToBP_MyCharacter (Game|GetPlayerCharacter 0)))
      (bind _output_get (Variables|Default|SetCharacterRef _asbp_my_character))
      (bind _move (Timeline|Move PlayFromStart)
        (:Update
          (Transformation|SetActorRelativeLocation (Math|Vector|Lerp(Vector) (Variables|Default|GetStart) (Variables|Default|GetEnd) _move)))
        (:Finished
          (bind _move_2 (Timeline|MoveBack ReverseFromEnd)
            (:Update
              (Transformation|SetActorRelativeLocation (Math|Vector|Lerp(Vector) (Variables|Default|GetStart) (Variables|Default|GetEnd) _move_2)))
            (:Finished
              (Timeline|Move PlayFromStart))))))
    (:Is%20Not%20Valid
      (Timeline|Move PlayFromStart))))

(event Collision|EventActorBeginOverlap
  (params (OtherActor :type Actor%20Object%20Reference)))

(event EventTick
  (params (DeltaSeconds :type Float%20%28single-precision%29)))

(fn ConstructionScript)